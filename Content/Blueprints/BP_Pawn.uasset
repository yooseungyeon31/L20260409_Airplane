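; BP_Pawn is a flyable pawn, apparently an aircraft, that constantly moves forward while the player steers its pitch and roll.
; Tick feeds the actor's forward vector into movement input at full scale, so changing orientation changes the direction of travel.
; The Pitch and Roll axes apply frame-rate-independent local rotations.
; A RotatePropeller helper spins a given component around its roll axis, but no graph here calls it.
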(event `self.ReceiveTick`
  (params (DeltaSeconds :type "Float (single-precision)"))
  (`self.AddMovementInput` (`self.GetActorForwardVector`)))

(event `InputAxis|Pitch`
  (params (AxisValue :type "Float (single-precision)"))
  (`self.K2_AddActorLocalRotation` (`KismetMathLibrary.MakeRotator` 0.0 (* AxisValue 60.0 (`GameplayStatics.GetWorldDeltaSeconds`)))))

(event `InputAxis|Roll`
  (params (AxisValue :type "Float (single-precision)"))
  (`self.K2_AddActorLocalRotation` (`KismetMathLibrary.MakeRotator` (* AxisValue 60.0 (`GameplayStatics.GetWorldDeltaSeconds`)))))

(fn `RotatePropeller`
  (params (Where :type "SceneComponent Object Reference") (RotationSpeed :type "Float (double-precision)"))
  (`SceneComponent.K2_AddLocalRotation` Where (`KismetMathLibrary.MakeRotator` (* (`GameplayStatics.GetWorldDeltaSeconds`) (`self.RotationSpeed`))) false false))

(fn `UserConstructionScript`)